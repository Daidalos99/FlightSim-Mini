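; BP_Plane is a player-controlled plane flown by throttle, roll, pitch and yaw axis inputs acting on its Fuselage component.
; Roll, Pitch and Yaw add frame-time-scaled local rotations, mapped respectively to the rotator's yaw, roll and pitch.
; Throttle adds actor location plus forward vector times ThrottleSpeed and input as a local offset, without delta time, and prints debug text.
; The constant forward movement on Tick is disabled.
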(event EventBeginPlay)

(event EventTick
  (params (DeltaSeconds :type Float%20%28single-precision%29))
  (Transformation|SetActorLocation (+ (Transformation|GetActorLocation) (* (Transformation|GetActorForwardVector) (* (Variables|Default|GetThrottleSpeed) DeltaSeconds))) false false))

(event Input|AxisEvents|InputAxisPitch
  (params (AxisValue :type Float%20%28single-precision%29))
  (if (!= AxisValue 0.0)
    (Transformation|AddLocalRotation (Variables|Default|Getfuselage) (Math|Rotator|MakeRotator (* AxisValue (* (Variables|Default|GetPitchSpeed) (Utilities|Time|GetWorldDeltaSeconds))) 0.0 0.0) false false)))

(event Input|AxisEvents|InputAxisYaw
  (params (AxisValue :type Float%20%28single-precision%29))
  (if (!= AxisValue 0.0)
    (Transformation|AddLocalRotation (Variables|Default|Getfuselage) (Math|Rotator|MakeRotator 0.0 (* AxisValue (* (Variables|Default|GetYawSpeed) (Utilities|Time|GetWorldDeltaSeconds))) 0.0) false false)))

(event Input|AxisEvents|InputAxisRoll
  (params (AxisValue :type Float%20%28single-precision%29))
  (if (!= AxisValue 0.0)
    (Transformation|AddLocalRotation (Variables|Default|Getfuselage) (Math|Rotator|MakeRotator 0.0 0.0 (* AxisValue (* (Variables|Default|GetRollSpeed) (Utilities|Time|GetWorldDeltaSeconds)))) false false)))

(event Input|AxisEvents|InputAxisThrottle
  (params (AxisValue :type Float%20%28single-precision%29))
  (bind _returnvalue (Transformation|GetActorForwardVector))
  (bind _throttlespeed (Variables|Default|GetThrottleSpeed))
  (bind _returnvalue_2 (* _returnvalue _throttlespeed))
  (if (!= AxisValue 0.0)
    (Class|SceneComponent|AddLocalTransform (Variables|Default|Getfuselage) (Math|Transform|MakeTransform (+ (Transformation|GetActorLocation) (* AxisValue _returnvalue_2)) "0, 0, 0" "1.000000,1.000000,1.000000") false false)
    (Development|PrintText (Utilities|Text|ToText(String) _returnvalue_2))))

(fn ConstructionScript)