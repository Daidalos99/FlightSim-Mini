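; BP_AirCraft is an aircraft steered through Throttle, Roll, Pitch and Yaw input axes.
; Roll, Pitch and Yaw add local rotation to the AirCraft component, scaled by axis value, per-axis speed and frame delta time.
; Throttle sets the actor location along its forward vector without sweep, but the vector is multiplied by zero, so it produces no movement.
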(event Input|AxisEvents|InputAxisPitch
  (params (AxisValue :type Float%20%28single-precision%29))
  (if (!= AxisValue 0.0)
    (Transformation|AddLocalRotation (Variables|Default|GetAirCraft) (Math|Rotator|MakeRotator 0.0 (* AxisValue (* (Variables|Default|GetPitch_Speed) (Utilities|Time|GetWorldDeltaSeconds))) 0.0) false false)))

(event Input|AxisEvents|InputAxisYaw
  (params (AxisValue :type Float%20%28single-precision%29))
  (if (!= AxisValue 0.0)
    (Transformation|AddLocalRotation (Variables|Default|GetAirCraft) (Math|Rotator|MakeRotator 0.0 0.0 (* AxisValue (* (Variables|Default|GetYaw_Speed) (Utilities|Time|GetWorldDeltaSeconds)))) false false)))

(event Input|AxisEvents|InputAxisRoll
  (params (AxisValue :type Float%20%28single-precision%29))
  (if (!= AxisValue 0.0)
    (Transformation|AddLocalRotation (Variables|Default|GetAirCraft) (Math|Rotator|MakeRotator (* AxisValue (* (Variables|Default|GetRoll_Speed) (Utilities|Time|GetWorldDeltaSeconds))) 0.0 0.0) false false)))

(event Input|AxisEvents|InputAxisThrottle
  (params (AxisValue :type Float%20%28single-precision%29))
  (if (!= AxisValue 0.0)
    (Transformation|SetActorLocation (+ (Transformation|GetActorLocation) (* (Transformation|GetActorForwardVector) "")) false false)))

(fn ConstructionScript)